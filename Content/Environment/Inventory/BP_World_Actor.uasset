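; BP_World_Actor represents an inventory item or quest in the world, with a widget label showing its name and amount.
; On BeginPlay, IsQuest selects either the quest name alone or the item's mesh and name, read from the class defaults of QuestSignature or ItemSignature.
; Both paths pass the name and Amount to WB_Item.
; Every Tick rotates the widget component toward the player character.
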(event `self.ReceiveBeginPlay`
  (if (`self.Is Quest`)
    (`self.Set Quest Name`)
    (else
      (`self.Set Item Mesh`)
      (`self.Set Item Name and Amount`))))

(event `self.ReceiveTick`
  (params (DeltaSeconds :type "Float (single-precision)"))
  (bind _wb_item (`self.WB_Item`))
  (`SceneComponent.K2_SetWorldRotation` _wb_item (`KismetMathLibrary.FindLookAtRotation` (`SceneComponent.K2_GetComponentLocation` _wb_item) (`SceneComponent.K2_GetComponentLocation` (`Actor.RootComponent` (`GameplayStatics.GetPlayerCharacter` 0)))) false false))

(fn `Set Item Mesh`
  (`StaticMeshComponent.SetStaticMesh` (`self.ItemMesh`) (`.ItemMesh_19_F69DE270460E472B81F1FF90FD1A2FC9` (break `/Game/Environment/Inventory/S_Item_Str` (defaults `Object` (`self.Item Signature`))))))

(fn `Set Item Name and Amount`
  (bind _aswb_item (cast `/Game/Environment/Inventory/Widgets/WB_Item` (`WidgetComponent.GetUserWidgetObject` (`self.WB_Item`))))
  (`/Game/Environment/Inventory/Widgets/WB_Item.Get Item Info` _aswb_item (break `/Game/Environment/Inventory/S_Item_Str` (defaults `Object` (`self.Item Signature`))) (`self.Amount`)))

(fn `Set Quest Name`
  (bind _aswb_item (cast `/Game/Environment/Inventory/Widgets/WB_Item` (`WidgetComponent.GetUserWidgetObject` (`self.WB_Item`))))
  (`/Game/Environment/Inventory/Widgets/WB_Item.Get Item Info` _aswb_item (break `/Game/Environment/QuestsSystem/S_Quest_Str` (defaults `Object` (`self.Quest Signature`))) (`self.Amount`)))

(fn `UserConstructionScript`)