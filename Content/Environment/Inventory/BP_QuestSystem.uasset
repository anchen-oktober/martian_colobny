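; Quest log Blueprint that stores quest classes in a fixed-size slot array, modeled on an inventory.
; It creates a WB_Quests widget on the player screen's main panel and refreshes individual widget slots when the array changes.
; AddQuest fills the first empty slot, and GetSlotData reads quest details from class defaults.
; Using a quest only prints a placeholder, and removal rewrites the slot with its existing value.
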(event `self.ReceiveBeginPlay`
  (`KismetArrayLibrary.Array_Resize` (`self.Slot Array`) (`self.Quests Amount`)))

(fn `Add Quest`
  (params (Quest :type "/Game/Environment/Inventory/BP_Master_Quest Class Reference") (Amount :type Integer :default 1))
  (returns (Success :type Boolean) (Result :type "/Game/Environment/Inventory/E_Add_Item_Result Enum"))
  (locals (`Empty Slot Index` :type Integer) (`Added Quest` :type "/Game/Environment/Inventory/BP_Master_Quest Class Reference"))
  (bind _empty_slot_index (`local.Empty Slot Index`))
  (set `local.Added Quest` Quest)
  (bind (_slot_found _found_slot_index) (`self.Find Empty Slot`))
  (if _slot_found
    (set `local.Empty Slot Index` _found_slot_index)
    (`KismetArrayLibrary.Array_Set` (`self.Slot Array`) _empty_slot_index (make `/Game/Environment/Inventory/S_QuestSlot_Str` (`local.Added Quest`) 1))
    (`self.Refresh Slot Data` _empty_slot_index)
    (return true "NewEnumerator4")
    (else
      (return false "NewEnumerator5"))))

(fn `Create WB Quests`
  (bind _returnvalue (`|CreateWidget` "/Game/Environment/Inventory/Widgets/WB_Quests.WB_Quests_C" null self))
  (set `self.WB Quests Ref` _returnvalue)
  (bind _returnvalue_2 (`CanvasPanel.AddChildToCanvas` (`/Game/Environment/UI/MainWinget_UI.MainPanel` (`self.Player Screen WB`)) (`self.WB Quests Ref`)))
  (`CanvasPanelSlot.SetAutoSize` _returnvalue_2 true)
  (`CanvasPanelSlot.SetPosition` _returnvalue_2 (960.0 420.0)))

(fn `Find Empty Slot`
  (returns (`Slot Found` :type Boolean) (`Found Slot index` :type Integer))
  (locals (`Empty Slot Found` :type Boolean))
  (for (_array_element _array_index) (`self.Slot Array`)
    (if (not (`KismetSystemLibrary.IsValidClass` (`.Quest_12_E46EF51849E53EED02A27F9604878DB5` (break `/Game/Environment/Inventory/S_QuestSlot_Str` _array_element))))
      (set `local.Empty Slot Found` true)
      (break)))
  (`KismetSystemLibrary.PrintString` "So what??")
  (return (`local.Empty Slot Found`) _array_index))

(fn `Get Slot Data`
  (params (Index :type Integer))
  (returns (Empty :type Boolean) (Quest :type "/Game/Environment/Inventory/S_Quest_Str Structure"))
  (bind _quest (break `/Game/Environment/Inventory/S_QuestSlot_Str` (`|GetArrayItem` (`self.Slot Array`) Index)))
  (if (`KismetSystemLibrary.IsValidClass` _quest)
    (return false (defaults `Object` _quest))
    (else
      (return true))))

(fn `Refresh Slot Data`
  (params (Index :type Integer))
  (`/Game/Environment/Inventory/Widgets/WB_QuestSlot.Update WB Quest Slot` (`|GetArrayItem` (`/Game/Environment/Inventory/Widgets/WB_Quests.WB Quests Slot Array` (`self.WB Quests Ref`)) Index)))

(fn `Remove Item in Index`
  (params (Index :type Integer))
  (locals (`Local Index` :type Integer))
  (bind _slot_array (`self.Slot Array`))
  (bind _local_index (`local.Local Index`))
  (set `local.Local Index` Index)
  (`KismetArrayLibrary.Array_Set` _slot_array _local_index (`|GetArrayItem` _slot_array _local_index))
  (`self.Refresh Slot Data` _local_index)
  (return))

(fn `UseQuest in Index`
  (params (Index :type Integer))
  (`KismetSystemLibrary.PrintString` "Quest does something" true true (struct :`R` 0.364583 :`B` 0.005315 :`A` 1.0)))

(fn `UserConstructionScript`)