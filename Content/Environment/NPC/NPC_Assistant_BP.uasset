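; Assistant NPC that displays a greeting in a world-space dialog widget when something enters its collision box.
; BeginPlay caches the widget component's user widget as an Assistant_Dialogs_UI reference.
; The box's begin-overlap event writes a hard-coded Russian greeting into that UI's text field, without filtering the overlapping actor.
; Tick rotates the widget component to face the first player's character every frame.
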(event `self.ReceiveBeginPlay`
  (bind _asassistant_dialogs_ui (cast `/Game/Environment/UI/Assistant_Dialogs_UI` (`WidgetComponent.GetUserWidgetObject` (`self.DialogsWidget`))))
  (set `self.As Assistant Dialogs UI` _asassistant_dialogs_ui))

(event `self.AssistantCollisionBox.OnComponentBeginOverlap`
  (params (OverlappedComponent :type "PrimitiveComponent Object Reference") (OtherActor :type "Actor Object Reference") (OtherComp :type "PrimitiveComponent Object Reference") (OtherBodyIndex :type Integer) (bFromSweep :type Boolean) (SweepResult :type "HitResult Structure (by ref)"))
  (`TextBlock.SetText` (`/Game/Environment/UI/Assistant_Dialogs_UI.DialogTextField` (`self.As Assistant Dialogs UI`)) "Здарова, чудик"))

(event `self.ReceiveTick`
  (params (DeltaSeconds :type "Float (single-precision)"))
  (`SceneComponent.K2_SetWorldRotation` (`self.DialogsWidget`) (`KismetMathLibrary.FindLookAtRotation` (`SceneComponent.K2_GetComponentLocation` (`self.DialogsWidget`)) (`SceneComponent.K2_GetComponentLocation` (`Actor.RootComponent` (`GameplayStatics.GetPlayerCharacter` 0)))) false false))

(fn `UserConstructionScript`)